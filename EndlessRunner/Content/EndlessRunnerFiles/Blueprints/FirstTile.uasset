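; Endless runner track tile that triggers the next tile's spawn when the character passes through its Box.
; The overlap also adds multiplied points, nudges player walk speed up within a clamp, then destroys the tile after a short delay.
; SpawnObstacles, not called in this graph, fills three lanes with pipes, boxes, coins or power-ups through chained, separately rolled chances.
; Some branches end early, and Boots checks on later lanes lack a random input.
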(event `self.Box.OnComponentBeginOverlap`
  (params (OverlappedComponent :type "PrimitiveComponent Object Reference") (OtherActor :type "Actor Object Reference") (OtherComp :type "PrimitiveComponent Object Reference") (OtherBodyIndex :type Integer) (bFromSweep :type Boolean) (SweepResult :type "HitResult Structure (by ref)"))
  (cast `/Game/EndlessRunnerFiles/Blueprints/ThirdPersonCharacter` OtherActor)
  (bind _asthird_person_game_mode (cast `/Game/ThirdPersonBP/Blueprints/ThirdPersonGameMode` (`GameplayStatics.GetGameMode`)))
  (`/Game/ThirdPersonBP/Blueprints/ThirdPersonGameMode.SpawnTile` _asthird_person_game_mode)
  (bind _asthird_person_game_mode_2 (cast `/Game/ThirdPersonBP/Blueprints/ThirdPersonGameMode` (`GameplayStatics.GetGameMode`)))
  (set `/Game/ThirdPersonBP/Blueprints/ThirdPersonGameMode.CurrentPoints` (+ (* 1 (`/Game/ThirdPersonBP/Blueprints/ThirdPersonGameMode.PointsMultiplier` _asthird_person_game_mode_2)) (`/Game/ThirdPersonBP/Blueprints/ThirdPersonGameMode.CurrentPoints` _asthird_person_game_mode_2)) _asthird_person_game_mode_2)
  (bind _asthird_person_character (cast `/Game/EndlessRunnerFiles/Blueprints/ThirdPersonCharacter` (`GameplayStatics.GetPlayerCharacter` 0)))
  (bind _charactermovement (`Character.CharacterMovement` _asthird_person_character))
  (set `CharacterMovementComponent.MaxWalkSpeed` (`KismetMathLibrary.FClamp` (* (`CharacterMovementComponent.MaxWalkSpeed` _charactermovement) 1.01) 100.0 2000.0) _charactermovement)
  (`KismetSystemLibrary.Delay` 0.5)
  (`self.K2_DestroyActor`))

(event `self.ReceiveBeginPlay`)

(fn `SpawnObstacles`
  (bind _returnvalue (`KismetMathLibrary.RandomFloatInRange` 0.0 1.0))
  (bind _returnvalue_2 (`KismetMathLibrary.RandomFloatInRange` 0.0 1.0))
  (bind _returnvalue_3 (`KismetMathLibrary.RandomFloatInRange` 0.0 1.0))
  (bind _returnvalue_4 (`SceneComponent.K2_GetComponentToWorld` (`self.Lane0`)))
  (bind _returnvalue_5 (`SceneComponent.K2_GetComponentToWorld` (`self.Lane1`)))
  (bind _returnvalue_6 (`SceneComponent.K2_GetComponentToWorld` (`self.Lane2`)))
  (if (`KismetMathLibrary.InRange_FloatFloat` _returnvalue 0.0 0.4)
    (`|SpawnActorFromClass` "/Game/EndlessRunnerFiles/Blueprints/Obstacle_Pipe.Obstacle_Pipe_C" _returnvalue_4 "Undefined" "OverrideRootScale" null null)
    (if (`KismetMathLibrary.InRange_FloatFloat` _returnvalue_2 0.0 0.4) :!label _label
      (`|SpawnActorFromClass` "/Game/EndlessRunnerFiles/Blueprints/Obstacle_Pipe.Obstacle_Pipe_C" _returnvalue_5 "Undefined" "OverrideRootScale" null null)
      (if (`KismetMathLibrary.InRange_FloatFloat` _returnvalue_3 0.0 0.4) :!label _label_2
        (`|SpawnActorFromClass` "/Game/EndlessRunnerFiles/Blueprints/Obstacle_Pipe.Obstacle_Pipe_C" _returnvalue_6 "Undefined" "OverrideRootScale" null null)
        (elif (`KismetMathLibrary.InRange_FloatFloat` _returnvalue_3 0.4 0.5)
          (`|SpawnActorFromClass` "/Game/EndlessRunnerFiles/Blueprints/Obstacle_Box.Obstacle_Box_C" _returnvalue_6 "Undefined" "OverrideRootScale" null null)
          (elif (`KismetMathLibrary.InRange_FloatFloat` _returnvalue_3 0.5 0.9)
            (`|SpawnActorFromClass` "/Game/EndlessRunnerFiles/Blueprints/Coin_pickUp.Coin_PickUp_C" _returnvalue_6 "Undefined" "OverrideRootScale" null null)
            (elif (`KismetMathLibrary.InRange_FloatFloat` _returnvalue_3 0.9 0.95)
              (`|SpawnActorFromClass` "/Game/EndlessRunnerFiles/Blueprints/Magnet_PickUp.Magnet_PickUp_C" _returnvalue_6 "Undefined" "OverrideRootScale" null null)
              (elif (`KismetMathLibrary.InRange_FloatFloat` 0.0 0.95)
                (`|SpawnActorFromClass` "/Game/EndlessRunnerFiles/Blueprints/Boots_PickUp.Boots_PickUp_C" _returnvalue_6 "Undefined" "OverrideRootScale" null null))))))
      (elif (`KismetMathLibrary.InRange_FloatFloat` _returnvalue_2 0.4 0.5)
        (`|SpawnActorFromClass` "/Game/EndlessRunnerFiles/Blueprints/Obstacle_Box.Obstacle_Box_C" _returnvalue_5 "Undefined" "OverrideRootScale" null null)
        (goto _label_2)
        (elif (`KismetMathLibrary.InRange_FloatFloat` _returnvalue_2 0.5 0.9)
          (`|SpawnActorFromClass` "/Game/EndlessRunnerFiles/Blueprints/Coin_pickUp.Coin_PickUp_C" _returnvalue_5 "Undefined" "OverrideRootScale" null null)
          (goto _label_2)
          (elif (`KismetMathLibrary.InRange_FloatFloat` _returnvalue_2 0.9 0.95)
            (`|SpawnActorFromClass` "/Game/EndlessRunnerFiles/Blueprints/Magnet_PickUp.Magnet_PickUp_C" _returnvalue_5 "Undefined" "OverrideRootScale" null null)
            (goto _label_2)
            (elif (`KismetMathLibrary.InRange_FloatFloat` 0.0 0.95)
              (`|SpawnActorFromClass` "/Game/EndlessRunnerFiles/Blueprints/Boots_PickUp.Boots_PickUp_C" _returnvalue_5 "Undefined" "OverrideRootScale" null null))))))
    (elif (`KismetMathLibrary.InRange_FloatFloat` _returnvalue 0.4 0.5)
      (`|SpawnActorFromClass` "/Game/EndlessRunnerFiles/Blueprints/Obstacle_Box.Obstacle_Box_C" _returnvalue_4 "Undefined" "OverrideRootScale" null null)
      (goto _label)
      (elif (`KismetMathLibrary.InRange_FloatFloat` _returnvalue 0.5 0.9)
        (`|SpawnActorFromClass` "/Game/EndlessRunnerFiles/Blueprints/Coin_pickUp.Coin_PickUp_C" _returnvalue_4 "Undefined" "OverrideRootScale" null null)
        (goto _label)
        (elif (`KismetMathLibrary.InRange_FloatFloat` _returnvalue 0.9 0.95)
          (`|SpawnActorFromClass` "/Game/EndlessRunnerFiles/Blueprints/Magnet_PickUp.Magnet_PickUp_C" _returnvalue_4 "Undefined" "OverrideRootScale" null null)
          (goto _label)
          (elif (`KismetMathLibrary.InRange_FloatFloat` _returnvalue 0.95 1.0)
            (`|SpawnActorFromClass` "/Game/EndlessRunnerFiles/Blueprints/Boots_PickUp.Boots_PickUp_C" _returnvalue_4 "Undefined" "OverrideRootScale" null null)))))))

(fn `UserConstructionScript`)